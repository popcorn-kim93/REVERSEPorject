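; Play HUD that draws an exit marker ("나가는곳") showing the player's distance in metres to the way out.
; On BeginPlay it stores the first actor tagged "OutWay" as NextStepActor.
; While DoView is true, DrawHUD projects that actor's location to the screen and draws the rounded distance centred just above it, with no check for off-screen targets.
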(event `self.ReceiveBeginPlay`
  (bind _outactors (`GameplayStatics.GetAllActorsWithTag` "OutWay"))
  (set `self.NextStepActor` (`|GetArrayItem` _outactors)))

(event `self.ReceiveDrawHUD`
  (params (SizeX :type Integer) (SizeY :type Integer))
  (bind _screenposition (`GameplayStatics.ProjectWorldToScreen` (`GameplayStatics.GetPlayerController` 0) (`self.K2_GetActorLocation` (`self.NextStepActor`))))
  (bind _returnvalue (`KismetStringLibrary.Concat_StrStr` "나가는곳 : " (`KismetStringLibrary.Conv_IntToString` (`KismetMathLibrary.Round` (/ (`KismetMathLibrary.VSize` (- (`self.K2_GetActorLocation` (`GameplayStatics.GetPlayerPawn` 0)) (`self.K2_GetActorLocation` (`self.NextStepActor`)))) 100.0))) "m"))
  (set `self.ScreenX` SizeX)
  (set `self.ScreenY` SizeY)
  (if (`self.DoView`)
    (`self.DrawText` _returnvalue (struct :`R` 0.588542 :`G` 0.566437 :`B` 0.587182 :`A` 1.0) (- (`KismetMathLibrary.BreakVector2D` _screenposition) (/ (`self.GetTextSize` _returnvalue "/Game/Fonts/Typo_SsangmunDongB__1__Font.Typo_SsangmunDongB__1__Font" 2.0) 2.0)) (+ (`.Y` (`KismetMathLibrary.BreakVector2D` _screenposition)) -50.0) "/Game/Fonts/Typo_SsangmunDongB__1__Font.Typo_SsangmunDongB__1__Font" 2.0)))

(fn `UserConstructionScript`)