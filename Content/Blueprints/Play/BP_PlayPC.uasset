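; BP_PlayPC is the gameplay player controller that manages the play-mode UI and player input.
; On BeginPlay it sets game-only input, caches BP_PlayHUD, shows the main widget and plays a timed loading-screen exit.
; Input actions toggle the HUD's view flag, signal restart press and release to the main widget and BP_PlayPawn, and toggle the menu.
; Separate functions pop up four tutorial widgets and a credits widget.
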(event `self.ReceiveBeginPlay`
  (bind _wb_loadingref (`self.WB_LoadingRef`))
  (`|ExecutionSequence`
    (:`then_0`
      (`WidgetBlueprintLibrary.SetInputMode_GameOnly` self)
      (set `self.bShowMouseCursor` false)
      (`/Engine/EditorBlueprintResources/StandardMacros.IsValid` (`self.WB_LoadingRef`) :!label _label
        (:`Is Valid`
          _)
        (:`Is Not Valid`
          (bind _returnvalue (`|CreateWidget` "/Game/UI/WB_Loading.WB_Loading_C"))
          (set `self.WB_LoadingRef` _returnvalue)))
      (bind _asbp_play_hud (cast `/Game/Blueprints/Play/BP_PlayHUD` (`self.GetHUD`)))
      (set `self.HudRef` _asbp_play_hud)
      (`/Engine/EditorBlueprintResources/StandardMacros.IsValid` (`self.WB_PlayMainRef`)
        (:`Is Valid`
          _)
        (:`Is Not Valid`
          (bind _returnvalue_2 (`|CreateWidget` "/Game/UI/Play/WB_PlayMain.WB_PlayMain_C"))
          (set `self.WB_PlayMainRef` _returnvalue_2)))
      (`UserWidget.AddToViewport` (`self.WB_PlayMainRef`) 0))
    (:`then_1`
      (goto _label))
    (:`then_2`
      (`UserWidget.AddToViewport` _wb_loadingref 0)
      (`/Game/UI/WB_Loading.WidgetOut` _wb_loadingref)
      (`KismetSystemLibrary.Delay` 6.0)
      (`Widget.RemoveFromParent` _wb_loadingref))))

(event `InputAction|K_ViewTarget`
  (params (Key :type "Key Structure"))
  (:`Pressed`
    (set `/Game/Blueprints/Play/BP_PlayHUD.DoView` true (`self.HudRef`)))
  (:`Released`
    (set `/Game/Blueprints/Play/BP_PlayHUD.DoView` false (`self.HudRef`))))

(event `InputAction|K_Restart`
  (params (Key :type "Key Structure"))
  (bind _wb_playmainref (`self.WB_PlayMainRef`))
  (bind _asbp_play_pawn (cast `/Game/Blueprints/Play/BP_PlayPawn` (`self.K2_GetPawn`) :!pure true))
  (:`Pressed`
    (`/Game/UI/Play/WB_PlayMain.DoRestarting` _wb_playmainref)
    (`/Game/Blueprints/Play/BP_PlayPawn.WantRestart` _asbp_play_pawn))
  (:`Released`
    (`/Game/UI/Play/WB_PlayMain.UndoRestarting` _wb_playmainref)
    (`/Game/Blueprints/Play/BP_PlayPawn.Want'nRestart` _asbp_play_pawn)))

(event `InputAction|K_Menu`
  (params (Key :type "Key Structure"))
  (bind _wb_playmainref (`self.WB_PlayMainRef`))
  (:`Pressed`
    (if (`/Game/UI/Play/WB_PlayMain.OnMenu` _wb_playmainref)
      (`/Game/UI/Play/WB_PlayMain.OutMenu` _wb_playmainref)
      (else
        (`/Game/UI/Play/WB_PlayMain.InMenu` _wb_playmainref)))))

(fn `1Tuto`
  (bind _returnvalue (`|CreateWidget` "/Game/UI/Play/WB_1Tuto.WB_1Tuto_C"))
  (`UserWidget.AddToViewport` _returnvalue 0))

(fn `2Tuto`
  (bind _returnvalue (`|CreateWidget` "/Game/UI/Play/WB_2Tuto.WB_2Tuto_C"))
  (`UserWidget.AddToViewport` _returnvalue 0))

(fn `3Tuto`
  (bind _returnvalue (`|CreateWidget` "/Game/UI/Play/WB_3Tuto.WB_3Tuto_C"))
  (`UserWidget.AddToViewport` _returnvalue 0))

(fn `4Tuto`
  (bind _returnvalue (`|CreateWidget` "/Game/UI/Play/WB_4Tuto.WB_4Tuto_C"))
  (`UserWidget.AddToViewport` _returnvalue 0))

(fn `CraditPop`
  (bind _returnvalue (`|CreateWidget` "/Game/UI/WB_Cradit.WB_Cradit_C"))
  (`UserWidget.AddToViewport` _returnvalue 0))

(fn `UserConstructionScript`)