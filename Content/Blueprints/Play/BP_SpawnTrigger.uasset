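; BP_SpawnTrigger is a trigger actor that launches a BP_Projectile from a random direction when a BP_PlayPawn enters its Box.
; Each overlap picks one of five distant spawn points around the trigger: overhead or along either side of the X and Y axes.
; Each spawn sets a fixed rotation per direction, with random lateral jitter on the four horizontal ones, and uses SpawnedScale for size.
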(event `self.Box.OnComponentBeginOverlap`
  (params (OverlappedComponent :type "PrimitiveComponent Object Reference") (OtherActor :type "Actor Object Reference") (OtherComp :type "PrimitiveComponent Object Reference") (OtherBodyIndex :type Integer) (bFromSweep :type Boolean) (SweepResult :type "HitResult Structure (by ref)"))
  (bind (_returnvalue_x _returnvalue_y _returnvalue_z) (`KismetMathLibrary.BreakVector` (`self.K2_GetActorLocation`)))
  (bind _spawnedscale (`self.SpawnedScale`))
  (bind _returnvalue (+ _returnvalue_z 200.0))
  (bind _returnvalue_2 (+ _returnvalue_y (`KismetMathLibrary.RandomFloatInRange` -100.0 100.0)))
  (bind _returnvalue_3 (+ _returnvalue_x (`KismetMathLibrary.RandomFloatInRange` -100.0 100.0)))
  (cast `/Game/Blueprints/Play/BP_PlayPawn` OtherActor)
  (switch `int` (`KismetMathLibrary.RandomIntegerInRange` 0 4)
    (:`0`
      (`KismetSystemLibrary.PrintString` "Top")
      (`|SpawnActorFromClass` "/Game/Blueprints/Play/BP_Projectile.BP_Projectile_C" (`KismetMathLibrary.MakeTransform` (`KismetMathLibrary.MakeVector` _returnvalue_x _returnvalue_y (+ _returnvalue_z 10000.0)) (struct :`Pitch` -90.0) _spawnedscale) "Undefined" "OverrideRootScale" null null))
    (:`1`
      (`KismetSystemLibrary.PrintString` "Back")
      (`|SpawnActorFromClass` "/Game/Blueprints/Play/BP_Projectile.BP_Projectile_C" (`KismetMathLibrary.MakeTransform` (`KismetMathLibrary.MakeVector` (- _returnvalue_x 10000.0) _returnvalue_2 _returnvalue) (struct) _spawnedscale) "Undefined" "OverrideRootScale" null null))
    (:`2`
      (`|SpawnActorFromClass` "/Game/Blueprints/Play/BP_Projectile.BP_Projectile_C" (`KismetMathLibrary.MakeTransform` (`KismetMathLibrary.MakeVector` (+ _returnvalue_x 10000.0) _returnvalue_2 _returnvalue) (struct :`Yaw` 180.0) _spawnedscale) "Undefined" "OverrideRootScale" null null))
    (:`3`
      (`|SpawnActorFromClass` "/Game/Blueprints/Play/BP_Projectile.BP_Projectile_C" (`KismetMathLibrary.MakeTransform` (`KismetMathLibrary.MakeVector` _returnvalue_3 (- _returnvalue_y 10000.0) _returnvalue) (struct :`Yaw` 90.0) _spawnedscale) "Undefined" "OverrideRootScale" null null))
    (:`4`
      (`|SpawnActorFromClass` "/Game/Blueprints/Play/BP_Projectile.BP_Projectile_C" (`KismetMathLibrary.MakeTransform` (`KismetMathLibrary.MakeVector` _returnvalue_3 (+ _returnvalue_y 10000.0) _returnvalue) (struct :`Yaw` -90.0) _spawnedscale) "Undefined" "OverrideRootScale" null null))))

(fn `UserConstructionScript`)