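; BP_ReverseGI, apparently the game instance by its name, handles the transition into the loading map.
; ShowLoading stores the destination level name, then creates the WB_Loading widget if needed, adds it to the viewport and plays WidgetIn.
; It increments DieCount on every call, then waits a fixed delay before opening Map_Loading rather than the destination itself.
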(event `ShowLoading`
  (params (MoveTo :type Name))
  (bind _wb_loading_ref (`self.WB_Loading_Ref`))
  (set `self.MoveLevelName` MoveTo)
  (`/Engine/EditorBlueprintResources/StandardMacros.IsValid` (`self.WB_Loading_Ref`)
    (:`Is Valid`
      _)
    (:`Is Not Valid`
      (bind _returnvalue (`|CreateWidget` "/Game/UI/WB_Loading.WB_Loading_C"))
      (set `self.WB_Loading_Ref` _returnvalue)))
  (`UserWidget.AddToViewport` _wb_loading_ref 0)
  (`/Game/UI/WB_Loading.WidgetIn` _wb_loading_ref)
  (set `self.DieCount` (+ (`self.DieCount`) 1))
  (`KismetSystemLibrary.Delay` 5.0)
  (`GameplayStatics.OpenLevel` "Map_Loading"))